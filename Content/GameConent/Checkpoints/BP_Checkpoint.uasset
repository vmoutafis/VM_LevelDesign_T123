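; BP_Checkpoint is a save checkpoint that activates when the player overlaps its trigger, then asks BP_GameInstance to save the game.
; Activation plays a sound and a timeline that raises the emissive power on a dynamic mesh material.
; On BeginPlay, unless saves are ignored, a saved checkpoint ID re-activates it and sends SaveCompleteMessage to related actors.
; GetSpawnTransform exposes a respawn location and rotation from its components.
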(event OnComponentBeginOverlap(Trigger)
  (params (OverlappedComponent :type Primitive%20Component%20Object%20Reference) (OtherActor :type Actor%20Object%20Reference) (OtherComp :type Primitive%20Component%20Object%20Reference) (OtherBodyIndex :type Integer) (bFromSweep :type Boolean) (SweepResult :type Hit%20Result%20Structure%20%28by%20ref%29))
  (if (and (== OtherActor (Game|GetPlayerCharacter 0)) (not (Variables|Default|GetbIsActive)))
    (CallFunction|ActivateCheckpoint)
    (Default|TrySaveGame (Variables|Default|GetGameInstance) self)))

(event Custom|Glow
  (bind _alpha (Timeline|TL_Glow Play)
    (:Update
      (Rendering|Material|SetScalarParameterValue (Variables|Default|GetMeshEmissiveMat) "EmissivePower" (Math|Float|Lerp 0.0 3.0 _alpha) :!class /Script/Engine.MaterialInstanceDynamic))))

(event EventBeginPlay
  (bind _asbp_game_instance (Utilities|Casting|CastToBP_GameInstance (Game|GetGameInstance)))
  (bind _output_get (Variables|Default|SetGameInstance _asbp_game_instance))
  (if (not (Variables|/Game/GameConent/Core/BP_GameInstance.BP_GameInstance_C|GetbIgnoreSave _output_get))
    (bind _savedgame (Variables|/Game/GameConent/Core/BP_GameInstance.BP_GameInstance_C|GetSavedGame (Variables|Default|GetGameInstance))
      (:then
        (if (Utilities|Array|ContainsItem (Variables|/Game/GameConent/Core/BP_SaveGame.BP_SaveGame_C|GetCheckpointIDs _savedgame) (Variables|Default|GetID))
          (CallFunction|ActivateCheckpoint)
          (for _array_element (Variables|Default|GetRelatedActorsToHandle)
            (Class|BISaveGameMechanics|SaveComplete(Message) _array_element))))
      (:else))))

(fn ConstructionScript
  (bind _returnvalue (Rendering|Material|CreateDynamicMaterialInstance (Variables|Default|GetStaticMesh) 0 (Rendering|Material|GetMaterial (Variables|Default|GetStaticMesh) 0) "None" :!class /Script/Engine.PrimitiveComponent))
  (Variables|Default|SetMeshEmissiveMat _returnvalue))

(fn ActivateCheckpoint
  (Variables|Default|SetbIsActive true)
  (CallFunction|Glow)
  (Audio|PlaySoundatLocation (Variables|Default|GetActivateSound) (Transformation|GetActorLocation) "0, 0, 0" 1.0 1.0 0.0 0 0 0 0))

(fn GetSpawnTransform
  (return (Math|Transform|MakeTransform (Transformation|GetWorldLocation (Variables|Default|GetSpawnLocation)) (Transformation|GetWorldRotation (Variables|Default|GetSpawnRotation)) "1.000000,1.000000,1.000000")))