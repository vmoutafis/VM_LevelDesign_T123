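; Actor component that tracks health for its owner, handling damage, healing and death.
; Binds the owner's point and radial damage events into one handler, which can optionally accept only player-caused damage, then clamps Health and calls the OnDamaged dispatcher.
; Non-player owners trigger the player HUD hit marker, flagging kills; IsDead updates afterwards, so the killing hit still registers.
; AddHealth restores clamped health and calls OnHeal.
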(event Custom|OnTakeRadialDamage
  (params (DamagedActor :type Actor%20Object%20Reference) (Damage :type Float%20%28single-precision%29) (DamageType :type Damage%20Type%20Object%20Reference) (Origin :type Vector) (HitInfo :type Hit%20Result%20Structure) (InstigatedBy :type Controller%20Object%20Reference) (DamageCauser :type Actor%20Object%20Reference))
  (CallFunction|HandleDamage Damage Origin DamageCauser))

(event Custom|OnTakeDamage
  (params (DamagedActor :type Actor%20Object%20Reference) (Damage :type Float%20%28single-precision%29) (InstigatedBy :type Controller%20Object%20Reference) (HitLocation :type Vector) (FHitComponent :type Primitive%20Component%20Object%20Reference) (BoneName :type Name) (ShotFromDirection :type Vector) (DamageType :type Damage%20Type%20Object%20Reference) (DamageCauser :type Actor%20Object%20Reference))
  (CallFunction|HandleDamage Damage HitLocation DamageCauser))

(event EventBeginPlay
  (EventDispatchers|BindEventtoOnTakePointDamage (Components|GetOwner) (EventDispatchers|CreateEvent :!event Custom|OnTakeDamage))
  (EventDispatchers|BindEventtoOnTakeRadialDamage (Components|GetOwner) (EventDispatchers|CreateEvent :!event Custom|OnTakeRadialDamage)))

(fn AddHealth
  (params (Amount :type Float%20%28double-precision%29))
  (Variables|Default|SetHealth (Math|Float|Clamp(Float) (+ (Variables|Default|GetHealth) Amount) 0.0 (Variables|Default|GetMaxHealth)))
  (Default|CallOnHeal Amount))

(fn HandleDamage
  (params (Damage :type Float%20%28double-precision%29) (Location :type Vector) (DamageCauser :type Actor%20Object%20Reference))
  (if (select (Variables|Default|GetbOnlyPlayer) (CallFunction|CheckIsPlayerCauser DamageCauser) true)
    (Variables|Default|SetDamageTaken Damage)
    (bind _output_get (Variables|Default|SetHealth (Math|Float|Clamp(Float) (- (Variables|Default|GetHealth) Damage) 0.0 (Variables|Default|GetMaxHealth))))
    (Default|CallOnDamaged (<= _output_get 0.0) (Variables|Default|GetDamageTaken) Location DamageCauser)
    (CallFunction|ActivateHitMarker)
    (Variables|Default|SetbIsDead (<= (Variables|Default|GetHealth) 0.0))))

(fn CheckIsPlayerCauser
  (params (Causer :type Actor%20Object%20Reference))
  (bind _returnvalue (Game|Player|GetPlayerPawn 0))
  (return (or (== Causer _returnvalue) (== _returnvalue (Components|GetOwner Causer)))))

(fn ActivateHitMarker
  (if (not (Variables|Default|GetbIsDead))
    (if (!= (Components|GetOwner) (Game|Player|GetPlayerPawn 0))
      (bind _asbp_first_person_character (Utilities|Casting|CastToBP_FirstPersonCharacter (Game|Player|GetPlayerPawn 0)))
      (Default|ActivateHitMarker (Variables|/Game/GameConent/Player/Blueprints/BP_FirstPersonCharacter.BP_FirstPersonCharacter_C|GetPlayerHUD _asbp_first_person_character) (<= (Variables|Default|GetHealth) 0.0)))))