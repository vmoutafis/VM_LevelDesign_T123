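; BP_Pickup is a generic spinning pickup, collected when player pawn 0 overlaps its trigger.
; Collection plays a sound and calls SetPickupEnabled, which toggles visibility, trigger collision and the decal's on/off material.
; Reusable pickups re-enable on a cooldown timer, while one-time pickups stay disabled and are also disabled on SaveComplete.
; Each pickup starts at a random yaw and rotates steadily on Tick.
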(event OnComponentBeginOverlap(Trigger)
  (params (OverlappedComponent :type Primitive%20Component%20Object%20Reference) (OtherActor :type Actor%20Object%20Reference) (OtherComp :type Primitive%20Component%20Object%20Reference) (OtherBodyIndex :type Integer) (bFromSweep :type Boolean) (SweepResult :type Hit%20Result%20Structure%20%28by%20ref%29))
  (if (== OtherActor (Game|Player|GetPlayerPawn 0))
    (CallFunction|PickupCollected OtherActor)))

(event EventSaveComplete
  (if (Variables|Pickup|GetbOneTimePickup)
    (CallFunction|SetPickupEnabled false)))

(event EventBeginPlay
  (CallFunction|RandomiseStartRotation))

(event EventTick
  (params (DeltaSeconds :type Float%20%28single-precision%29))
  (Transformation|AddRelativeRotation (Variables|Default|GetTransform) (Math|Rotator|MakeRotator 0.0 0.0 (* DeltaSeconds -1.5e+02)) false false))

(fn ConstructionScript
  (Rendering|Components|Decal|SetDecalMaterial (Variables|Default|GetDecal) (Variables|Default|GetDecalMaterialOn)))

(fn SetPickupEnabled
  (params (bEnabled :type Boolean))
  (Rendering|SetVisibility (Variables|Default|GetTransform) bEnabled true)
  (Collision|SetCollisionEnabled (Variables|Default|GetTrigger) (select bEnabled "QueryOnly" "NoCollision"))
  (Rendering|Components|Decal|SetDecalMaterial (Variables|Default|GetDecal) (select bEnabled (Variables|Default|GetDecalMaterialOn) (Variables|Default|GetDecalMaterialOff))))

(fn PickupCollected
  (params (OtherActor :type Actor%20Object%20Reference))
  (Audio|PlaySoundatLocation (Variables|Pickup|GetPickupAudio) (Transformation|GetActorLocation) "0, 0, 0" 1.0 1.0 0.0 0 0 0 0)
  (CallFunction|SetPickupEnabled false)
  (if (not (Variables|Pickup|GetbOneTimePickup))
    (Utilities|Time|SetTimerbyFunctionName 0 "ReEnable" (Variables|Pickup|GetCooldown))))

(fn ReEnable
  (CallFunction|SetPickupEnabled true))

(fn RandomiseStartRotation
  (Transformation|SetRelativeRotation (Variables|Default|GetTransform) (Math|Rotator|MakeRotator 0.0 0.0 (Math|Random|RandomFloatinRange 0.0 3.6e+02)) false false))