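; Actor component on BP_FirstPersonCharacter that tracks collected keys, collectables and a special key inventory.
; Add functions update these values and the player HUD, which also refreshes once its loaded event fires.
; Show flags gate HUD updates, except in AddSpecialKey; hidden key and collectable displays are removed only on updates after that first load.
; Adding a special key also calls TryUnlockDoor on every BP_Door with the key's tag.
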(event Custom|PlayerHudLoaded
  (CallFunction|UpdateKeysUI)
  (CallFunction|UpdateCollectablesUI)
  (CallFunction|UpdateSpecialKeysUI)
  (Variables|Default|SetbFirstLoad true))

(event EventBeginPlay
  (bind _asbp_first_person_character (Utilities|Casting|CastToBP_FirstPersonCharacter (Components|GetOwner)))
  (EventDispatchers|BindEventtoPlayerHUDLoaded _asbp_first_person_character (EventDispatchers|CreateEvent :!event Custom|PlayerHudLoaded)))

(fn AddKey
  (params (Amount :type Integer))
  (Variables|Default|SetKeysCollected (+ (Variables|Default|GetKeysCollected) Amount))
  (CallFunction|UpdateKeysUI))

(fn AddCollectable
  (params (Amount :type Integer))
  (Variables|Default|SetCollectablesCollected (+ (Variables|Default|GetCollectablesCollected) Amount))
  (CallFunction|UpdateCollectablesUI))

(fn UpdateKeysUI
  (if (Variables|Default|GetbShowKeysUI)
    (bind _asbp_first_person_character (Utilities|Casting|CastToBP_FirstPersonCharacter (Components|GetOwner)))
    (bind _playerhud (Variables|/Game/GameConent/Player/Blueprints/BP_FirstPersonCharacter.BP_FirstPersonCharacter_C|GetPlayerHUD _asbp_first_person_character)
      (:then
        (Default|UpdateNormalKeyUI _playerhud (Variables|Default|GetKeysCollected)))
      (:else))
    (elif (Variables|Default|GetbFirstLoad)
      (bind _asbp_first_person_character_2 (Utilities|Casting|CastToBP_FirstPersonCharacter (Components|GetOwner)))
      (bind _playerhud_2 (Variables|/Game/GameConent/Player/Blueprints/BP_FirstPersonCharacter.BP_FirstPersonCharacter_C|GetPlayerHUD _asbp_first_person_character_2)
        (:then
          (Default|RemoveKeys _playerhud_2))
        (:else)))))

(fn UpdateCollectablesUI
  (if (Variables|Default|GetbShowCollectablesUI)
    (bind _asbp_first_person_character (Utilities|Casting|CastToBP_FirstPersonCharacter (Components|GetOwner)))
    (bind _playerhud (Variables|/Game/GameConent/Player/Blueprints/BP_FirstPersonCharacter.BP_FirstPersonCharacter_C|GetPlayerHUD _asbp_first_person_character)
      (:then
        (Default|UpdateOtherCollectableUI _playerhud (Variables|Default|GetCollectablesCollected)))
      (:else))
    (elif (Variables|Default|GetbFirstLoad)
      (bind _asbp_first_person_character_2 (Utilities|Casting|CastToBP_FirstPersonCharacter (Components|GetOwner)))
      (bind _playerhud_2 (Variables|/Game/GameConent/Player/Blueprints/BP_FirstPersonCharacter.BP_FirstPersonCharacter_C|GetPlayerHUD _asbp_first_person_character_2)
        (:then
          (Default|RemoveCollectables _playerhud_2))
        (:else)))))

(fn AddSpecialKey
  (params (Key :type ST%20Special%20Key%20Inventory%20Structure%20%28by%20ref%29))
  (Utilities|Array|Add (Variables|Default|GetSpecialKeyInventory) Key)
  (bind _outactors (Actor|GetAllActorsOfClass "/Game/GameConent/GameplayMechanics/Doors/BP_Door.BP_Door_C"))
  (for _array_element _outactors
    (Default|TryUnlockDoor _array_element (.Tag (Utilities|Struct|BreakST_SpecialKeyInventory Key))))
  (bind _asbp_first_person_character (Utilities|Casting|CastToBP_FirstPersonCharacter (Components|GetOwner)))
  (bind _playerhud (Variables|/Game/GameConent/Player/Blueprints/BP_FirstPersonCharacter.BP_FirstPersonCharacter_C|GetPlayerHUD _asbp_first_person_character)
    (:then
      (Default|UpdateSpecialKeysUI _playerhud (Variables|Default|GetSpecialKeyInventory)))
    (:else)))

(fn UpdateSpecialKeysUI
  (if (Variables|Default|GetbShowSpecialKeysUI)
    (bind _asbp_first_person_character (Utilities|Casting|CastToBP_FirstPersonCharacter (Components|GetOwner)))
    (bind _playerhud (Variables|/Game/GameConent/Player/Blueprints/BP_FirstPersonCharacter.BP_FirstPersonCharacter_C|GetPlayerHUD _asbp_first_person_character)
      (:then
        (Default|UpdateSpecialKeysUI _playerhud (Variables|Default|GetSpecialKeyInventory)))
      (:else))))