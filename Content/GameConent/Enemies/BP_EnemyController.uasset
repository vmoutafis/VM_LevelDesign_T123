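; Enemy AI controller that runs a behavior tree and targets the player once perceived.
; The construction script starts the tree, and BeginPlay stores the controller's own location as StartLocation in the blackboard.
; When AI perception successfully senses the first player's pawn, SetEnemyTarget writes it to TargetActor and passes it to the controlled pawn through a message call.
; Nothing here clears the target when sensing is lost.
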(event OnTargetPerceptionUpdated(AIPerception)
  (params (Actor :type Actor%20Object%20Reference) (Stimulus :type AI%20Stimulus%20Structure))
  (if (and (== Actor (Game|Player|GetPlayerPawn 0)) (Utilities|Struct|BreakAIStimulus Stimulus))
    (CallFunction|SetEnemyTarget Actor)))

(event EventBeginPlay
  (AI|Components|Blackboard|SetValueasVector (AI|GetBlackboard 0) (Utilities|Name|MakeLiteralName "StartLocation") (Transformation|GetActorLocation)))

(event EventTick
  (params (DeltaSeconds :type Float%20%28single-precision%29)))

(fn ConstructionScript
  (AI|RunBehaviorTree (Variables|Default|GetBehaviourTree)))

(fn SetEnemyTarget
  (params (Actor :type Actor%20Object%20Reference))
  (bind _output_get (LocalVariables|SetLTarget Actor))
  (AI|Components|Blackboard|SetValueasObject (AI|GetBlackboard 0) (Utilities|Name|MakeLiteralName "TargetActor") _output_get)
  (Class|BIEnemies|EnemeySetEnemyTarget(Message) (Pawn|GetControlledPawn) (LocalVariables|GetLTarget))
  (return))