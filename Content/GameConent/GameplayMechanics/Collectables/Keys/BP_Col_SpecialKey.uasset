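; Colour-tagged special key collectable that the first-person character can pick up.
; The construction script creates a dynamic material instance and uses the ColourTag to set its emissive tint and the point light to red, green, blue or yellow.
; On collection it passes its class and tag to the character, then destroys itself.
; A separate AddCollectable function records the same class and tag in the game instance.
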(event EventBeginPlay)

(event Collision|EventActorBeginOverlap
  (params (OtherActor :type Actor%20Object%20Reference)))

(event EventTick
  (params (DeltaSeconds :type Float%20%28single-precision%29)))

(fn ConstructionScript
  (bind _colourtag (Variables|SpecialKey|GetColourTag))
  (bind _returnvalue (Utilities|Select :Index _colourtag :NewEnumerator0 "(R=1.000000,G=0.000000,B=0.000000,A=1.000000)" :NewEnumerator1 "(R=0.000000,G=1.000000,B=0.000000,A=1.000000)" :NewEnumerator2 "(R=0.000000,G=0.000000,B=0.500000,A=1.000000)" :NewEnumerator3 "(R=1.000000,G=1.000000,B=0.000000,A=1.000000)"))
  (|CallParentFunction)
  (CallFunction|SetMatInstance)
  (bind _matinstance (Variables|Default|GetMatInstance)
    (:then
      (Rendering|Material|SetVectorParameterValue _matinstance "EmissiveTint" _returnvalue :!class /Script/Engine.MaterialInstanceDynamic)
      (Rendering|Components|Light|SetLightColor (Variables|Default|GetPointLight) _returnvalue true))
    (:else)))

(fn OnCollect
  (params (Actor :type Actor%20Object%20Reference))
  (bind _asbp_first_person_character (Utilities|Casting|CastToBP_FirstPersonCharacter Actor))
  (Default|AddSpecialKey _asbp_first_person_character (Utilities|Struct|MakeST_SpecialKeyInventory (Utilities|GetClass self) (Variables|SpecialKey|GetColourTag)))
  (Actor|DestroyActor))

(fn AddCollectable
  (params (CollectableComponent :type AC%20Collectables%20Object%20Reference))
  (bind _asbp_game_instance (Utilities|Casting|CastToBP_GameInstance (Game|GetGameInstance)))
  (Default|AddSpecialKey _asbp_game_instance (Utilities|Struct|MakeST_SpecialKeyInventory (Utilities|GetClass self) (Variables|SpecialKey|GetColourTag))))

(fn SetMatInstance
  (bind _staticmesh (Variables|Default|GetStaticMesh))
  (bind _returnvalue (Rendering|Material|GetMaterial _staticmesh 0))
  (if (and (Utilities|IsValid _staticmesh) (Utilities|IsValid _returnvalue))
    (bind _returnvalue_2 (Rendering|Material|CreateDynamicMaterialInstance _staticmesh 0 _returnvalue "None" :!class /Script/Engine.PrimitiveComponent))
    (Variables|Default|SetMatInstance _returnvalue_2)))