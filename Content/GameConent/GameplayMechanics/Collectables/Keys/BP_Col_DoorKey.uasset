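; Door key collectable that feeds keys to doors when an actor collects it.
; OnCollect runs the parent collect logic, then adds its Value as keys to each door in its Doors array.
; It then finds every BP_Door in the level and calls TryUnlockDoor on each with a fixed enum value, including doors outside that array.
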(event EventBeginPlay
  (|CallParentFunction) ; This node is disabled and will not be called.\nDrag off pins to build functionality.
)

(event Collision|EventActorBeginOverlap
  (params (OtherActor :type Actor%20Object%20Reference)))

(event EventTick
  (params (DeltaSeconds :type Float%20%28single-precision%29))
  (|CallParentFunction DeltaSeconds) ; This node is disabled and will not be called.\nDrag off pins to build functionality.
)

(fn ConstructionScript
  (|CallParentFunction))

(fn OnCollect
  (params (Actor :type Actor%20Object%20Reference))
  (|CallParentFunction Actor)
  (for _array_element (Variables|DoorKey|GetDoors)
    (Default|AddKeys _array_element (Variables|DoorKey|GetValue)))
  (bind _outactors (Actor|GetAllActorsOfClass "/Game/GameConent/GameplayMechanics/Doors/BP_Door.BP_Door_C"))
  (for _array_element_2 _outactors
    (Default|TryUnlockDoor _array_element_2 "NewEnumerator0")))