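; BP_Col_Simple is a simple collectable that awards points when collected.
; It overrides AddCollectable, calling the parent version and then passing its CollectableValue to AddCollectablePoints on BP_GameInstance.
; The event graph holds only disabled placeholder events, and the construction script just calls its parent.
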(event EventBeginPlay
  (|CallParentFunction) ; This node is disabled and will not be called.\nDrag off pins to build functionality.
)

(event Collision|EventActorBeginOverlap
  (params (OtherActor :type Actor%20Object%20Reference)))

(event EventTick
  (params (DeltaSeconds :type Float%20%28single-precision%29))
  (|CallParentFunction DeltaSeconds) ; This node is disabled and will not be called.\nDrag off pins to build functionality.
)

(fn ConstructionScript
  (|CallParentFunction))

(fn AddCollectable
  (params (CollectableComponent :type AC%20Collectables%20Object%20Reference))
  (|CallParentFunction CollectableComponent)
  (bind _asbp_game_instance (Utilities|Casting|CastToBP_GameInstance (Game|GetGameInstance)))
  (Default|AddCollectablePoints _asbp_game_instance (Variables|Default|GetCollectableValue)))