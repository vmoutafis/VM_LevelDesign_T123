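; Base collectable pickup that can spin from a random yaw and bob on a randomly offset timeline.
; Unless blocked, any actor overlapping the trigger plays a sound, credits player 0's AC_Collectables if the item counts, then calls OnCollect, which destroys it.
; AddCollectable and OnCollect are separate functions from the main Collect flow, and a SaveComplete event also destroys the actor.
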(event OnComponentBeginOverlap(Trigger)
  (params (OverlappedComponent :type Primitive%20Component%20Object%20Reference) (OtherActor :type Actor%20Object%20Reference) (OtherComp :type Primitive%20Component%20Object%20Reference) (OtherBodyIndex :type Integer) (bFromSweep :type Boolean) (SweepResult :type Hit%20Result%20Structure%20%28by%20ref%29))
  (if (not (Variables|Collectable|GetbCantBeCollected))
    (CallFunction|Collect OtherActor)))

(event EventTick
  (params (DeltaSeconds :type Float%20%28single-precision%29))
  (if (Variables|Collectable|GetbShouldSpin)
    (Transformation|AddRelativeRotation (Variables|Default|GetTransform) (Math|Rotator|MakeRotator 0.0 0.0 (* DeltaSeconds (Variables|Collectable|GetRotationSpeed))) false false)))

(event EventBeginPlay
  (CallFunction|RandomiseStartRotation)
  (if (Variables|Collectable|GetbShouldFloat)
    (Utilities|FlowControl|Sequence
      (:then_0
        (bind _alpha (Timeline|TL_Float SetNewTime)
          (:Update
            (Transformation|SetRelativeLocation (Variables|Default|GetTransform) (Math|Vector|MakeVector 0.0 0.0 (Math|Float|Lerp -1e+01 1e+01 _alpha)) false false))))
      (:then_1
        (Timeline|TL_Float Play)))))

(event EventSaveComplete
  (Actor|DestroyActor))

(fn ConstructionScript)

(fn Collect
  (params (Actor :type Actor%20Object%20Reference))
  (Audio|PlaySoundatLocation (Variables|Collectable|GetCollectSound) (Transformation|GetActorLocation) "0, 0, 0" 1.0 1.0 0.0 0 0 0 0)
  (CallFunction|ApplyCollectable)
  (CallFunction|OnCollect Actor))

(fn OnCollect
  (params (Actor :type Actor%20Object%20Reference))
  (Actor|DestroyActor))

(fn AddCollectable
  (params (CollectableComponent :type AC%20Collectables%20Object%20Reference))
  (Default|AddCollectable CollectableComponent (Variables|Collectable|GetCollectableValue)))

(fn ApplyCollectable
  (bind _returnvalue (Game|Player|GetPlayerPawn 0))
  (bind _returnvalue_2 (Actor|GetComponentbyClass _returnvalue "/Game/GameConent/Player/Blueprints/AC_Collectables.AC_Collectables_C"))
  (if (and (Variables|Collectable|GetbCountAsCollectable) (Utilities|IsValid _returnvalue_2))
    (CallFunction|AddCollectable _returnvalue_2)))

(fn RandomiseStartRotation
  (if (Variables|Collectable|GetbShouldSpin)
    (Transformation|SetRelativeRotation (Variables|Default|GetTransform) (Math|Rotator|MakeRotator 0.0 0.0 (Math|Random|RandomFloatinRange 0.0 3.6e+02)) false false)))