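; Base door actor that gates opening behind key counts or a tagged special key, with optional open-on-play and trigger-driven auto open/close.
; TryOpen checks either the interacting first-person character's special key inventory or a key count, held locally or globally in the player's AC_Collectables.
; ForceAccess, set on SaveComplete, bypasses those checks.
; Open and Close only set IsOpen, and the key-collected hooks are empty, leaving visible behaviour to be implemented elsewhere.
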(event OnComponentBeginOverlap(DoorAutoTrigger)
  (params (OverlappedComponent :type Primitive%20Component%20Object%20Reference) (OtherActor :type Actor%20Object%20Reference) (OtherComp :type Primitive%20Component%20Object%20Reference) (OtherBodyIndex :type Integer) (bFromSweep :type Boolean) (SweepResult :type Hit%20Result%20Structure%20%28by%20ref%29))
  (Variables|Default|SetInteractedActor OtherActor)
  (if (CallFunction|PlayerCondition OtherActor)
    (if (Variables|Door|GetbAutoOpen/Close)
      (CallFunction|TryOpen))))

(event OnComponentEndOverlap(DoorAutoTrigger)
  (params (OverlappedComponent :type Primitive%20Component%20Object%20Reference) (OtherActor :type Actor%20Object%20Reference) (OtherComp :type Primitive%20Component%20Object%20Reference) (OtherBodyIndex :type Integer))
  (Variables|Default|SetInteractedActor OtherActor)
  (if (CallFunction|PlayerCondition OtherActor)
    (if (Variables|Door|GetbAutoOpen/Close)
      (CallFunction|TryClose))))

(event EventBeginPlay
  (if (Variables|Door|GetbOpenOnPlay)
    (CallFunction|Open)))

(event EventSaveComplete
  (Variables|Door|SetbForceAccess true))

(fn ConstructionScript)

(fn Open
  (Variables|Default|SetbIsOpen true))

(fn Close
  (Variables|Default|SetbIsOpen false))

(fn PlayerCondition
  (params (OtherActor :type Object%20Object%20Reference))
  (return (or (== OtherActor (Game|Player|GetPlayerPawn 0)) (not (Variables|Door|GetbOnlyPlayer)))))

(fn HasCollectedKeys
  (bind _returnvalue (Game|Player|GetPlayerPawn 0))
  (bind _returnvalue_2 (Actor|GetComponentbyClass _returnvalue "/Game/GameConent/Player/Blueprints/AC_Collectables.AC_Collectables_C"))
  (LocalVariables|SetLCollectablesComponent _returnvalue_2)
  (if (and (Utilities|IsValid _returnvalue_2) (Variables|LockedDoors|GetbUseGlobalKeys))
    (return (>= (Variables|/Game/GameConent/Player/Blueprints/AC_Collectables.AC_Collectables_C|GetKeysCollected (LocalVariables|GetLCollectablesComponent)) (Variables|LockedDoors|GetKeysOrEnemiesToUnlock)))
    (else
      (return (>= (Variables|Default|GetKeysCollected) (Variables|LockedDoors|GetKeysOrEnemiesToUnlock))))))

(fn AddKey
  (Math|Integer|IncrementInt (Variables|Default|GetKeysCollected)
    (:%20%20
      (if (Variables|LockedDoors|GetbOpenOnUnlock)
        (CallFunction|TryOpen)))))

(fn AddKeys
  (params (KeysCollected :type Integer))
  (Variables|Default|SetKeysCollected (+ (Variables|Default|GetKeysCollected) KeysCollected))
  (if (Variables|LockedDoors|GetbOpenOnUnlock)
    (CallFunction|TryOpen)))

(fn TryOpen
  (if (not (Variables|Door|GetbForceAccess))
    (if (select (Variables|SpecialKey|GetbUseSpecialKey) (CallFunction|PlayerHasSpecialKey) (CallFunction|HasCollectedKeys))
      (if (not (Variables|Default|GetbIsOpen))
        (CallFunction|Open)))
    (else
      (CallFunction|Open))))

(fn TryClose
  (if (Variables|Door|GetbCanClose)
    (if (Variables|Default|GetbIsOpen)
      (CallFunction|Close))))

(fn ToggleDoor
  (if (Variables|Default|GetbIsOpen)
    (CallFunction|TryClose)
    (else
      (CallFunction|TryOpen))))

(fn RemoveKey
  (params (Amount :type Integer))
  (Variables|Default|SetKeysCollected (Math|Integer|Max(Integer) (- (Variables|Default|GetKeysCollected) Amount)))
  (if (not (CallFunction|HasCollectedKeys))
    (CallFunction|TryClose)))

(fn PlayerHasSpecialKey
  (bind _asbp_first_person_character (Utilities|Casting|CastToBP_FirstPersonCharacter (Variables|Default|GetInteractedActor))
    (:then
      (bind _array_element (Utilities|Array|ForEachLoopwithBreak (Variables|/Game/GameConent/Player/Blueprints/AC_Collectables.AC_Collectables_C|GetSpecialKeyInventory (Variables|/Game/GameConent/Player/Blueprints/BP_FirstPersonCharacter.BP_FirstPersonCharacter_C|GetAC_Collectables _asbp_first_person_character)) :!label _label)
        (:LoopBody
          (if (Utilities|Enum|Equal(Enum) (Utilities|Struct|BreakST_SpecialKeyInventory _array_element) (Variables|SpecialKey|GetSpecialKeyTag))
            (LocalVariables|SetLHasSpecialKey true)
            (goto _label Break)))
        (:Completed
          (return (LocalVariables|GetLHasSpecialKey)))))
    (:CastFailed
      (return false))))

(fn IsUnlocked
  (return (or (select (Variables|SpecialKey|GetbUseSpecialKey) (CallFunction|PlayerHasSpecialKey) (CallFunction|HasCollectedKeys)) (Variables|Door|GetbForceAccess))))

(fn TryUnlockDoor
  (params (SpecialKeyTag :type E_SpecialKeyColours%20Enum :default "NewEnumerator0"))
  (if (Variables|SpecialKey|GetbUseSpecialKey)
    (if (Utilities|Enum|Equal(Enum) SpecialKeyTag (Variables|SpecialKey|GetSpecialKeyTag))
      (CallFunction|OnSpecialKeyCollected))
    (elif (CallFunction|IsUnlocked)
      (CallFunction|OnKeysCollected))))

(fn OnSpecialKeyCollected)

(fn OnKeysCollected)