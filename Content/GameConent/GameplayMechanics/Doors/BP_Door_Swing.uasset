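; BP_Door_Swing is a child door Blueprint that swings open and closed by rotating in yaw.
; Its Open and Close overrides call the parent, then trigger SlideOpen and SlideClosed events, which play a sound and run one timeline forward or in reverse.
; The timeline's alpha lerps relative rotation toward RotationAngle, with play rate set on BeginPlay from TimeToOpen.
; Timeline and event names refer to sliding and rise/lower, though the motion is rotational.
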(event Custom|SlideClosed
  (Audio|PlaySoundatLocation (Variables|SwingDoor|GetCloseSound) (Transformation|GetActorLocation) "0, 0, 0" 1.0 1.0 0.0 0 0 0 0)
  (bind _alpha (Timeline|TL_RiseLower Reverse)
    (:Update
      (Transformation|SetRelativeRotation (Variables|Default|GetTransform) (Math|Rotator|Lerp(Rotator) "0, 0, 0" (Math|Rotator|MakeRotator 0.0 0.0 (Variables|SwingDoor|GetRotationAngle)) _alpha) false false))))

(event Custom|SlideOpen
  (Audio|PlaySoundatLocation (Variables|SwingDoor|GetOpenSound) (Transformation|GetActorLocation) "0, 0, 0" 1.0 1.0 0.0 0 0 0 0)
  (bind _alpha (Timeline|TL_RiseLower Play)
    (:Update
      (Transformation|SetRelativeRotation (Variables|Default|GetTransform) (Math|Rotator|Lerp(Rotator) "0, 0, 0" (Math|Rotator|MakeRotator 0.0 0.0 (Variables|SwingDoor|GetRotationAngle)) _alpha) false false))))

(event EventBeginPlay
  (|CallParentFunction)
  (Components|Timeline|SetPlayRate (Variables|Default|GetTL_RiseLower) (/ 1.0 (Variables|SwingDoor|GetTimeToOpen))))

(fn ConstructionScript
  (|CallParentFunction))

(fn Open
  (|CallParentFunction)
  (CallFunction|SlideOpen))

(fn Close
  (|CallParentFunction)
  (CallFunction|SlideClosed))