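; Base Blueprint for interactable objects that add or remove keys on linked doors and activate connected interactables.
; Interact either fires once or toggles HasInteracted, calling the empty OnInteract hook before propagating; ReleaseInteract calls the empty OnRelease hook.
; Connected interactables receive IgnoreTrigger set to true, so they skip their own doors and connections, preventing chain reactions.
; The SaveComplete event also runs a full Interact.
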(event EventSaveComplete
  (CallFunction|Interact false))

(fn ConstructionScript)

(fn TriggerDoors
  (bind _doorstoopen (Variables|Interactable|GetDoorsToOpen))
  (if (not (Variables|Default|GetbHasInteracted))
    (for _array_element _doorstoopen
      (Default|AddKey _array_element))
    (else
      (for _array_element_2 _doorstoopen
        (Default|RemoveKey _array_element_2 1)))))

(fn Interact
  (params (bIgnoreTrigger :type Boolean))
  (Variables|Default|SetbIgnoreTrigger bIgnoreTrigger)
  (if (Variables|Interactable|GetbInteractOnce)
    (if (not (Variables|Default|GetbHasInteracted))
      (CallFunction|OnInteract)
      (CallFunction|ActivateOtherInteractables)
      (CallFunction|TriggerMechanics)
      (Variables|Default|SetbHasInteracted true))
    (else
      (CallFunction|OnInteract)
      (CallFunction|ActivateOtherInteractables)
      (CallFunction|TriggerMechanics)
      (Variables|Default|SetbHasInteracted (not (Variables|Default|GetbHasInteracted))))))

(fn ReleaseInteract
  (params (bIgnoreTrigger :type Boolean))
  (Variables|Default|SetbIgnoreTrigger bIgnoreTrigger)
  (CallFunction|OnRelease))

(fn OnInteract)

(fn TriggerMechanics
  (if (not (Variables|Default|GetbIgnoreTrigger))
    (CallFunction|TriggerDoors)))

(fn ActivateOtherInteractables
  (if (not (Variables|Default|GetbIgnoreTrigger))
    (for _array_element (Variables|Interactable|GetConnectedInteractables)
      (CallFunction|Interact _array_element true))))

(fn OnRelease)