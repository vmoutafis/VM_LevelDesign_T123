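; Cog switch interactable that switches on or off on interaction, with a swinging arm, colour feedback and sound.
; OnInteract calls the parent, then branches on HasInteracted to play or reverse a timeline that rotates the arm and to play the matching optional sound.
; SetLightActive sets both the point light and the emissive tint of a dynamic material instance to the active or inactive colour.
; The construction script creates that instance and applies the initial colour from HasInteracted.
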(event Custom|ActivateArm
  (CallFunction|SetLightActive true)
  (bind _alpha (Timeline|TL_RotateArm Play)
    (:Update
      (Transformation|SetRelativeRotation (Variables|Default|GetArmTransform) (Math|Rotator|Lerp(Rotator) "0.000000,0.000000,-55.000000" "0.000000,0.000000,55.000000" _alpha true) false false))))

(event Custom|DeactivateArm
  (CallFunction|SetLightActive false)
  (bind _alpha (Timeline|TL_RotateArm Reverse)
    (:Update
      (Transformation|SetRelativeRotation (Variables|Default|GetArmTransform) (Math|Rotator|Lerp(Rotator) "0.000000,0.000000,-55.000000" "0.000000,0.000000,55.000000" _alpha true) false false))))

(fn ConstructionScript
  (|CallParentFunction)
  (CallFunction|SetBaseMatInstance)
  (CallFunction|SetLightActive (Variables|Default|GetbHasInteracted)))

(fn OnInteract
  (bind _returnvalue (Transformation|GetActorLocation))
  (|CallParentFunction)
  (if (not (Variables|Default|GetbHasInteracted))
    (CallFunction|ActivateArm)
    (bind _switchactivesound (Variables|Switch|GetSwitchActiveSound)
      (:then
        (Audio|PlaySoundatLocation _switchactivesound _returnvalue "0, 0, 0" 1.0 1.0 0.0 0 0 0 0))
      (:else))
    (else
      (CallFunction|DeactivateArm)
      (bind _switchinactivesound (Variables|Switch|GetSwitchInactiveSound)
        (:then
          (Audio|PlaySoundatLocation _switchinactivesound _returnvalue "0, 0, 0" 1.0 1.0 0.0 0 0 0 0))
        (:else)))))

(fn SetLightActive
  (params (bActive :type Boolean))
  (Rendering|Components|Light|SetLightColor (Variables|Default|GetPointLight) (Math|Color|SelectColor (Variables|Switch|GetActiveColour) (Variables|Switch|GetInactiveColour) bActive) true)
  (Rendering|Material|SetVectorParameterValue (Variables|Default|GetBaseMatInstance) "EmissiveTint" (Math|Color|SelectColor (Variables|Switch|GetActiveColour) (Variables|Switch|GetInactiveColour) bActive) :!class /Script/Engine.MaterialInstanceDynamic))

(fn SetBaseMatInstance
  (bind _staticmesh (Variables|Default|GetStaticMesh))
  (bind _returnvalue (Rendering|Material|GetMaterial _staticmesh 0))
  (if (and (Utilities|IsValid _staticmesh) (Utilities|IsValid _returnvalue))
    (bind _returnvalue_2 (Rendering|Material|CreateDynamicMaterialInstance _staticmesh 0 _returnvalue "None" :!class /Script/Engine.PrimitiveComponent))
    (Variables|Default|SetBaseMatInstance _returnvalue_2)))