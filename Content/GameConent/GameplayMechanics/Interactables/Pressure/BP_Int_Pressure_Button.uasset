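; Pressure button interactable that sinks when interacted with and rises when released, extending its parent's OnInteract and OnRelease.
; A timeline lowers the button transform by a set drop amount and plays in reverse on release, with an optional sound for each direction.
; The construction script creates dynamic material instances for both meshes, whose emissive tint switches between active and inactive colours with the pressed state.
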(event Custom|ButtonDown
  (CallFunction|PlaySoundifValid (Variables|PressureButton|GetButtonDownSound))
  (CallFunction|ChangeLightColour true)
  (bind _alpha (Timeline|TL_ButtonDownUp Play)
    (:Update
      (Transformation|SetRelativeLocation (Variables|Default|GetButtonTransform) (Math|Vector|MakeVector 0.0 0.0 (Math|Float|Lerp 0.0 (* (Variables|PressureButton|GetButtonDropAmount) -1.0) _alpha)) false false))))

(event Custom|ButtonUp
  (CallFunction|PlaySoundifValid (Variables|PressureButton|GetButtonUpSound))
  (CallFunction|ChangeLightColour false)
  (bind _alpha (Timeline|TL_ButtonDownUp Reverse)
    (:Update
      (Transformation|SetRelativeLocation (Variables|Default|GetButtonTransform) (Math|Vector|MakeVector 0.0 0.0 (Math|Float|Lerp 0.0 (* (Variables|PressureButton|GetButtonDropAmount) -1.0) _alpha)) false false))))

(fn ConstructionScript
  (|CallParentFunction)
  (CallFunction|CreateMatInstancefromMesh (Variables|Default|GetButton))
  (CallFunction|CreateMatInstancefromMesh (Variables|Default|GetStaticMesh))
  (CallFunction|ChangeLightColour false))

(fn OnInteract
  (|CallParentFunction)
  (CallFunction|ButtonDown))

(fn OnRelease
  (|CallParentFunction)
  (CallFunction|ButtonUp))

(fn ChangeLightColour
  (params (bIsActive :type Boolean))
  (for _array_element (Variables|Default|GetMaterialInstances)
    (Rendering|Material|SetVectorParameterValue _array_element "EmissiveTint" (Math|Color|SelectColor (Variables|PressureButton|GetActiveColour) (Variables|PressureButton|GetInactiveColour) bIsActive) :!class /Script/Engine.MaterialInstanceDynamic))
  (return))

(fn CreateMatInstancefromMesh
  (params (MeshComponent :type Primitive%20Component%20Object%20Reference))
  (bind _returnvalue (Rendering|Material|GetMaterial MeshComponent 0))
  (if (and (Utilities|IsValid MeshComponent) (Utilities|IsValid _returnvalue))
    (bind _returnvalue_2 (Rendering|Material|CreateDynamicMaterialInstance MeshComponent 0 _returnvalue "None" :!class /Script/Engine.PrimitiveComponent))
    (Utilities|Array|Add (Variables|Default|GetMaterialInstances) _returnvalue_2)))

(fn PlaySoundifValid
  (params (Sound :type Sound%20Base%20Object%20Reference))
  (Utilities|IsValid Sound
    (:Is%20Valid
      (Audio|PlaySoundatLocation Sound (Transformation|GetActorLocation) "0, 0, 0" 1.0 1.0 0.0 0 0 0 0))))