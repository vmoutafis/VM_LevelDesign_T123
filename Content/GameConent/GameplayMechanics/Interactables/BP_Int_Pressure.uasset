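; BP_Int_Pressure is a pressure-style interactable that activates when the player or an allowed physics object overlaps its trigger.
; Physics objects qualify by component tag or simulated physics, and IgnorePlayer makes the trigger ignore a collision channel.
; Interact is skipped when both player and object are inside; release requires both absent, ReverseOnExit set and InteractOnce off.
; OnRelease fires TriggerMechanics again and clears HasInteracted.
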(event OnComponentBeginOverlap(Trigger)
  (params (OverlappedComponent :type Primitive%20Component%20Object%20Reference) (OtherActor :type Actor%20Object%20Reference) (OtherComp :type Primitive%20Component%20Object%20Reference) (OtherBodyIndex :type Integer) (bFromSweep :type Boolean) (SweepResult :type Hit%20Result%20Structure%20%28by%20ref%29))
  (if (and (CallFunction|IsCorrectPhysicsObject OtherComp) (Variables|Pressure|GetbAllowPhysicsObject))
    (CallFunction|Interact false)
    (elif (== OtherActor (Game|Player|GetPlayerPawn 0))
      (CallFunction|Interact false))))

(event OnComponentEndOverlap(Trigger)
  (params (OverlappedComponent :type Primitive%20Component%20Object%20Reference) (OtherActor :type Actor%20Object%20Reference) (OtherComp :type Primitive%20Component%20Object%20Reference) (OtherBodyIndex :type Integer))
  (if (and (CallFunction|IsCorrectPhysicsObject OtherComp) (Variables|Pressure|GetbAllowPhysicsObject))
    (CallFunction|ReleaseInteract false)
    (elif (== OtherActor (Game|Player|GetPlayerPawn 0))
      (CallFunction|ReleaseInteract false))))

(event EventBeginPlay
  (|CallParentFunction)
  (if (Variables|Pressure|GetbIgnorePlayer)
    (Collision|SetCollisionResponsetoChannel (Variables|Default|GetTrigger) "ECC_GameTraceChannel3" "ECR_Ignore")))

(fn ConstructionScript
  (|CallParentFunction)
  (if (not (Variables|Pressure|GetbUseOnlyPhysicsObjectTag))
    (Variables|Pressure|SetPhysicsObjectTag "None")))

(fn ReleaseInteract
  (params (bIgnoreTrigger :type Boolean))
  (if (and (not (CallFunction|IsPlayerinTrigger)) (not (CallFunction|IsPhysicsObjectinTrigger)))
    (if (and (not (Variables|Default|GetbInteractOnce)) (Variables|Pressure|GetbReverseOnExit))
      (|CallParentFunction bIgnoreTrigger))))

(fn IsPhysicsObjectinTrigger
  (bind _array_element (Utilities|Array|ForEachLoopwithBreak (Class|PrimitiveComponent|GetOverlappingComponents (Variables|Default|GetTrigger)) :!label _label)
    (:LoopBody
      (if (CallFunction|IsCorrectPhysicsObject _array_element)
        (LocalVariables|SetbIsInTrigger true)
        (goto _label Break)))
    (:Completed
      (return (LocalVariables|GetbIsInTrigger)))))

(fn Interact
  (params (bIgnoreTrigger :type Boolean))
  (if (or (not (CallFunction|IsPlayerinTrigger)) (not (CallFunction|IsPhysicsObjectinTrigger)))
    (|CallParentFunction bIgnoreTrigger)))

(fn IsPlayerinTrigger
  (return (Utilities|Array|ContainsItem (Collision|GetOverlappingActors (Variables|Default|GetTrigger) 0 :!class /Script/Engine.PrimitiveComponent) (Game|Player|GetPlayerPawn 0))))

(fn IsCorrectPhysicsObject
  (params (Component :type Scene%20Component%20Object%20Reference))
  (return (select (Variables|Pressure|GetbUseOnlyPhysicsObjectTag) (Components|ComponentHasTag Component (Variables|Pressure|GetPhysicsObjectTag)) (Class|SceneComponent|IsAnySimulatingPhysics Component))))

(fn OnRelease
  (|CallParentFunction)
  (CallFunction|TriggerMechanics)
  (Variables|Default|SetbHasInteracted false))