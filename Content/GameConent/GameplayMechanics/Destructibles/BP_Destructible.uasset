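; Destructible actor that is destroyed when its AC_Health component reports lethal damage.
; The damage event sets a one-time Destroyed flag, stores the damage causer and calls EndLife, which simply destroys the actor.
; A separate SaveComplete event also destroys the actor directly, bypassing EndLife and the flag.
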(event OnDamaged(AC_Health)
  (params (bDead :type Boolean) (Damage :type Float%20%28double-precision%29) (HitLocation :type Vector :default "0, 0, 0") (DamageCauser :type Actor%20Object%20Reference))
  (if (and bDead (not (Variables|Default|GetbDestroyed)))
    (Variables|Default|SetbDestroyed true)
    (Variables|Default|SetDamageCauser DamageCauser)
    (CallFunction|EndLife)))

(event EventSaveComplete
  (Actor|DestroyActor))

(fn ConstructionScript)

(fn EndLife
  (Actor|DestroyActor))