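; Explosive destructible that deals full radial damage within its Range sphere when its life ends, then plays effects and sound and destroys itself.
; The construction script multiplies the damage by one plus the count of other BP_Des_Explode actors overlapping Range.
; The explosion effect prefers Niagara and falls back to a particle emitter.
; A separate Knockback function launches a given character horizontally away from the actor.
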(event EventBeginPlay)

(event Collision|EventActorBeginOverlap
  (params (OtherActor :type Actor%20Object%20Reference)))

(event EventTick
  (params (DeltaSeconds :type Float%20%28single-precision%29)))

(fn ConstructionScript
  (bind _range (Variables|Default|GetRange))
  (|CallParentFunction)
  (Variables|Explosion|SetCurrentDamage (Variables|Explosion|GetExplosionDamage))
  (bind _outactors (Collision|ComponentOverlapActors _range (Transformation|GetWorldTransform _range) (Utilities|Array|MakeArray "ObjectTypeQuery2") "BP_Des_Explode_C" (Utilities|Array|MakeArray self)))
  (Variables|Explosion|SetCurrentDamage (* (Variables|Explosion|GetCurrentDamage) (+ (Utilities|Array|Length _outactors) 1))))

(fn EndLife
  (Game|Damage|ApplyRadialDamage (Variables|Explosion|GetCurrentDamage) (Transformation|GetActorLocation) (Components|Sphere|GetScaledSphereRadius (Variables|Default|GetRange)) 0 0 self 0 true "ECC_WorldStatic")
  (CallFunction|SpawnExplosionifSet)
  (Audio|PlaySoundatLocation (Variables|Default|GetExplosionSound) (Transformation|GetActorLocation) "0, 0, 0" 1.0 1.0 0.0 0 0 0 0)
  (Actor|DestroyActor))

(fn SpawnExplosionifSet
  (bind _returnvalue (Transformation|GetActorLocation))
  (bind _explosionparticlescale (Variables|Default|GetExplosionParticleScale))
  (bind _explosionniagara (Variables|Explosion|GetExplosionNiagara)
    (:then
      (Niagara|SpawnSystematLocation _explosionniagara _returnvalue "0, 0, 0" _explosionparticlescale))
    (:else
      (bind _explosionparticle (Variables|Explosion|GetExplosionParticle)
        (:then
          (Effects|SpawnEmitteratLocation _explosionparticle _returnvalue "0, 0, 0" _explosionparticlescale))
        (:else)))))

(fn Knockback
  (params (Actor :type Actor%20Object%20Reference))
  (bind _returnvalue (Transformation|GetActorLocation))
  (bind _returnvalue_2 (Transformation|GetActorLocation Actor))
  (bind _knockbackamount (Variables|Default|GetKnockbackAmount))
  (bind _returnvalue_3 (Math|Rotator|FindLookatRotation _returnvalue _returnvalue_2))
  (bind _returnvalue_4 (Math|Vector|GetForwardVector _returnvalue_3))
  (bind _returnvalue_5 (* _returnvalue_4 _knockbackamount))
  (bind _ascharacter (Utilities|Casting|CastToCharacter Actor))
  (Character|LaunchCharacter _ascharacter (Math|Vector|MakeVector (.x _returnvalue_5) (.y _returnvalue_5) 0.0) true false))