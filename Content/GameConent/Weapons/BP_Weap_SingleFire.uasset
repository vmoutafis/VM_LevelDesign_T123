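; BP_Weap_SingleFire is a semi-automatic weapon child Blueprint that overrides its parent's firing functions.
; FirePressed calls the parent only when refire is allowed, then locks firing until a FireRate timer calls AllowRefire.
; ShootProjectile runs the parent logic, then, with a valid character, spawns a damage-carrying rifle projectile at SpawnLoc.
; It also plays hip or iron-sight rifle arm montages, a pistol weapon montage and pistol camera shake.
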(event EventBeginPlay
  (|CallParentFunction) ; This node is disabled and will not be called.\nDrag off pins to build functionality.
)

(event Collision|EventActorBeginOverlap
  (params (OtherActor :type Actor%20Object%20Reference)))

(event EventTick
  (params (DeltaSeconds :type Float%20%28single-precision%29)))

(fn ConstructionScript
  (|CallParentFunction))

(fn ShootProjectile
  (|CallParentFunction)
  (bind _fpscharref (Variables|Default|GetFPSCharRef)
    (:then
      (Animation|Montage|MontagePlay (Default|GetArmsAnimInstance _fpscharref) (select (Variables|Default|GetbIronSight) "/Game/FPS_Assault_Pack/Animations/Rifle/A_Arms_Rifle_Isight_Shoot01_Montage.A_Arms_Rifle_Isight_Shoot01_Montage" "/Game/FPS_Assault_Pack/Animations/Rifle/A_Arms_Rifle_Shoot01_Montage.A_Arms_Rifle_Shoot01_Montage") 1.0 "Duration" 0.0 true)
      (Game|SpawnActorfromClass "/Game/GameConent/Weapons/Projectiles/Projectile_P_Rifle.Projectile_P_Rifle_C" (Transformation|GetWorldTransform (Variables|Default|GetSpawnLoc)) "AlwaysSpawn" (Components|GetOwner) (Variables|Default|GetDamage) 0)
      (bind _camerashakesource (Class|BIPlayer|PlayerGetCameraShakeSource(Message) (Components|GetOwner)))
      (CameraShakes|StartCameraShake _camerashakesource "/Game/GameConent/Core/CameraShakes/CS_Pistol.CS_Pistol_C" 1.0 "World" "0, 0, 0")
      (Animation|Montage|MontagePlay (Components|SkeletalMesh|GetAnimInstance (Variables|Default|GetSkeletalMeshComponent)) "/Game/SciFiWeapDark/Weapons/Anims/Fire_Pistol_W_Montage.Fire_Pistol_W_Montage" 1.0 "Duration" 0.0 true))
    (:else)))

(fn FirePressed
  (if (Variables|Default|GetbRefireAllowed)
    (|CallParentFunction)
    (Variables|Default|SetbRefireAllowed false)
    (Utilities|Time|SetTimerbyFunctionName 0 "AllowRefire" (Variables|Default|GetFireRate))))

(fn AllowRefire
  (Variables|Default|SetbRefireAllowed true))