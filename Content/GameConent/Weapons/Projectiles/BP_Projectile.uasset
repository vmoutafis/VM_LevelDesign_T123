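; BP_Projectile is a weapon projectile that damages the first actor it overlaps other than its owner.
; On overlap it applies point damage, using its own location and forward vector to build the hit result and naming its owner as damage causer.
; It then calls EndLife, a separate function that destroys the projectile.
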(event Collision|EventActorBeginOverlap
  (params (OtherActor :type Actor%20Object%20Reference))
  (bind _returnvalue (Transformation|GetActorLocation))
  (bind _returnvalue_2 (Transformation|GetActorForwardVector))
  (Variables|Default|SetHitActor OtherActor)
  (if (!= OtherActor (Components|GetOwner))
    (Game|Damage|ApplyPointDamage (Variables|Default|GetHitActor) (Variables|Default|GetDamage) (Transformation|GetActorForwardVector) (Collision|MakeHitResult false false 0.0 0.0 _returnvalue _returnvalue _returnvalue_2 _returnvalue_2 0 0) 0 (Components|GetOwner) (Variables|Default|GetDamageClass))
    (CallFunction|EndLife)))

(fn ConstructionScript)

(fn EndLife
  (Actor|DestroyActor))