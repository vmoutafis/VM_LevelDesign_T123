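; Automatic weapon Blueprint that repeats the parent's fire action while fire is held.
; FirePressed starts a looping OnAutoFire timer at FireRate, with a negative start delay so the first shot is near-immediate.
; A DelayRefire timer gates re-pressing, and presses during that cooldown schedule a retry that fires only if HoldingFire is set.
; FireReleased calls the parent's release and clears the auto-fire loop.
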(event EventBeginPlay
  (|CallParentFunction) ; This node is disabled and will not be called.\nDrag off pins to build functionality.
)

(event Collision|EventActorBeginOverlap
  (params (OtherActor :type Actor%20Object%20Reference)))

(event EventTick
  (params (DeltaSeconds :type Float%20%28single-precision%29)))

(fn ConstructionScript
  (|CallParentFunction))

(fn FirePressed
  (bind _firerate (Variables|Default|GetFireRate))
  (if (Variables|Default|GetbRefireAllowed)
    (if (Variables|Default|GetbHoldingFire)
      (Utilities|Time|SetTimerbyFunctionName 0 "OnAutoFire" _firerate true (* _firerate -1.0))
      (Utilities|Time|SetTimerbyFunctionName 0 "DelayRefire" (Variables|Default|GetFireRate))
      (Variables|Default|SetbRefireAllowed false))
    (else
      (Utilities|Time|SetTimerbyFunctionName 0 "FirePressed" (Variables|Default|GetFireRate)))))

(fn OnAutoFire
  (|CallParentFunction))

(fn FireReleased
  (|CallParentFunction)
  (Utilities|Time|ClearTimerbyFunctionName 0 "OnAutoFire"))

(fn DelayRefire
  (Variables|Default|SetbRefireAllowed true))